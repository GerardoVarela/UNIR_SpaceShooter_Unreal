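; BP_EnemyH is a space shooter enemy that sets side-to-side movement, starting in a random direction and building on its parent Blueprint's behavior.
; SetMovementDirection flips IsRight and sets MovementVector from the actor's right vector, keeping only the negated Y component for the opposite direction.
; Overlapping an actor tagged "Lateral" reverses the direction and updates DelayShot, tying shot timing to each bounce.
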(event Custom|SetMovementDirection
  (bind _returnvalue (Transformation|GetActorRightVector))
  ;[0.15 0.15 0.15 0.5] Movement Direction
  (if (Variables|Default|GetIsRight)
    (Variables|Default|SetIsRight false)
    (Variables|Default|SetMovementVector (* _returnvalue "0.000000,-1.000000,0.000000"))
    (else
      (Variables|Default|SetIsRight true)
      (Variables|Default|SetMovementVector _returnvalue))))

(event EventBeginPlay
  ;[0.15 0.15 0.15 0.5] Set Random Direction at Start
  (|CallParentFunction)
  (Variables|Default|SetIsRight (Math|Random|RandomBool))
  (CallFunction|SetMovementDirection))

(event Collision|EventActorBeginOverlap
  (params (OtherActor :type Actor%20Object%20Reference))
  ;[0.15 0.15 0.15 0.5] Movement From Left to Right and Delay Shoot
  (|CallParentFunction OtherActor)
  (if (Actor|ActorHasTag OtherActor "Lateral")
    (CallFunction|SetMovementDirection)
    (Variables|Default|SetDelayShot (- (>= (Variables|Default|GetDelayShot) 0.2) 0.1))))

(event EventTick
  (params (DeltaSeconds :type Float%20%28single-precision%29))
  (|CallParentFunction DeltaSeconds) ; This node is disabled and will not be called.\nDrag off pins to build functionality.
)

(fn ConstructionScript
  (|CallParentFunction))