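; BP_SpaceS_EnemyAmmo is an enemy projectile for the space shooter.
; Each tick it moves along its forward vector at Speed, without sweeping.
; On overlap with any actor other than a BP_EnemyBase, it destroys itself after a short delay, applying no damage itself.
; An explosion particle and sound chain is present but disconnected, so it never runs.
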(event EventBeginPlay)

(event Collision|EventActorBeginOverlap
  (params (OtherActor :type Actor%20Object%20Reference))
  (Utilities|Casting|CastToBP_EnemyBase OtherActor
    (:CastFailed
      (Utilities|FlowControl|Delay 0.1)
      (Actor|DestroyActor))))

(event EventTick
  (params (DeltaSeconds :type Float%20%28single-precision%29))
  (Transformation|SetActorLocation (+ (Transformation|GetActorLocation) (* (Transformation|GetActorForwardVector) (* DeltaSeconds (Variables|Default|GetSpeed)))) false false))

(fn ConstructionScript)