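; BP_EnemyTriple is a space shooter enemy worth 3 that moves in a zigzag pattern.
; On BeginPlay it calls its parent, then sets its value and a diagonal MovementVector.
; Tick starts ChangeDirection whenever none is pending, so the vector's Y component flips every half second through a boolean-guarded Delay loop.
; Tick also calls the parent, which is left to handle everything else.
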(event Custom|ChangeDirection
  (Variables|Default|SetUpdatingDirection true)
  (Utilities|FlowControl|Delay 0.5)
  (Variables|Default|SetMovementVector (* (Variables|Default|GetMovementVector) "1.000000,-1.000000,0.000000"))
  (Variables|Default|SetUpdatingDirection false))

(event EventBeginPlay
  (|CallParentFunction)
  (Variables|Default|SetEnemyValue 3)
  (Variables|Default|SetMovementVector "-0.500000,0.250000,0.000000"))

(event Collision|EventActorBeginOverlap
  (params (OtherActor :type Actor%20Object%20Reference))
  (|CallParentFunction OtherActor) ; This node is disabled and will not be called.\nDrag off pins to build functionality.
)

(event EventTick
  (params (DeltaSeconds :type Float%20%28single-precision%29))
  (if (Variables|Default|GetUpdatingDirection)
    _
    (else
      (CallFunction|ChangeDirection)))
  (|CallParentFunction DeltaSeconds))

(fn ConstructionScript
  (|CallParentFunction))