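; Space shooter spawner actor that periodically drops a random powerup into the level.
; On BeginPlay a looping timer fires every SpawnTime seconds and calls SpawnPowerup.
; GetClassToSpawn picks BP_SpaceS_Powerup or BP_SpaceS_Reactor from a random index bounded by MaxNumPowerups.
; SpawnPowerup places it at a random scene component tagged "SpawnPoint", adjusting for collisions but always spawning.
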(event Custom|Spawn
  (CallFunction|SpawnPowerup))

(event EventBeginPlay
  (Utilities|Time|SetTimerbyEvent (delegate Custom|Spawn) (Variables|Default|GetSpawnTime) true))

(event Collision|EventActorBeginOverlap
  (params (OtherActor :type Actor%20Object%20Reference)))

(event EventTick
  (params (DeltaSeconds :type Float%20%28single-precision%29)))

(fn ConstructionScript)

(fn SpawnPowerup
  (bind _returnvalue (Actor|GetComponentsbyTag "/Script/Engine.SceneComponent" "SpawnPoint"))
  (bind _class (CallFunction|GetClasstoSpawn))
  (bind _returnvalue_2 (Game|SpawnActorfromClass _class (Transformation|GetWorldTransform (Utilities|Array|Get(acopy) _returnvalue (Math|Random|RandomInteger (Utilities|Array|Length _returnvalue)))) "AdjustIfPossibleButAlwaysSpawn" "MultiplyWithRoot" 0 0))
  (return _returnvalue_2))

(fn GetClasstoSpawn
  (return (Utilities|Select :Index (Math|Random|RandomInteger (Variables|Default|GetMaxNumPowerups)) :Option%200 "/Game/SpaceShooter/Players/BP_SpaceS_Powerup.BP_SpaceS_Powerup_C" :Option%201 "/Game/SpaceShooter/Players/BP_SpaceS_Reactor.BP_SpaceS_Reactor_C")))