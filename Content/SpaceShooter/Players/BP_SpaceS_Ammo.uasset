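; Player projectile for the space shooter that flies along its forward vector every tick.
; While the player character's powerup is active, it first scales up its capsule on a timeline, pinned just ahead of the FirePoint, before launching.
; Overlapping anything other than a Pawn or a Heart- or Reactor-tagged actor spawns an explosion with sound, then destroys it after a short delay.
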(event Custom|IncreaseAmmo
  ;[0.15 0.15 0.15 0.5] Increase Ammo
  (bind _scalealpha (Timeline|ScaleAmmoTimeline Play)
    (:Update
      (Transformation|SetWorldScale3D (Variables|Default|GetCapsule) (Math|Vector|MakeVector _scalealpha _scalealpha _scalealpha))
      (Transformation|SetActorLocation (+ (Transformation|GetWorldLocation (Variables|/Game/SpaceShooter/Players/BP_SpaceS_Character.BP_SpaceS_Character_C|GetFirePoint (Variables|Default|Getm_PlayerCharacter))) "30.000000,0.000000,0.000000") false false))
    (:Finished
      (Variables|Default|SetIncreasingDone true))))

(event EventBeginPlay
  ;[0.15 0.15 0.15 0.5] Get Character Reference
  (bind _asbp_space_s_character (Utilities|Casting|CastToBP_SpaceS_Character (Game|GetPlayerCharacter 0)))
  (Variables|Default|Setm_PlayerCharacter _asbp_space_s_character))

(event Collision|EventActorBeginOverlap
  (params (OtherActor :type Actor%20Object%20Reference))
  ;[0.15 0.15 0.15 0.5] Explode On Hit
  (Utilities|Casting|CastToPawn OtherActor
    (:CastFailed
      (if (not (or (Actor|ActorHasTag OtherActor "Heart") (Actor|ActorHasTag OtherActor "Reactor")))
        (Effects|SpawnEmitteratLocation "/Game/StarterContent/Particles/P_Explosion.P_Explosion" (Transformation|GetActorLocation))
        (Audio|PlaySound2D "/Game/SpaceShooter/Sounds/SS_Enemy_Explosion.SS_Enemy_Explosion" 0.7 1.0 0.0 0 0)
        (Utilities|FlowControl|Delay 0.1)
        (Actor|DestroyActor)))))

(event EventTick
  (params (DeltaSeconds :type Float%20%28single-precision%29))
  ;[0.15 0.15 0.15 0.5] Move Ammo
  (if (and (Variables|/Game/SpaceShooter/Players/BP_SpaceS_Character.BP_SpaceS_Character_C|GetPowerupActivated (Variables|Default|Getm_PlayerCharacter)) (== (Variables|Default|GetIncreasingDone) false))
    (CallFunction|IncreaseAmmo)
    (else
      (Transformation|SetActorLocation (+ (Transformation|GetActorLocation) (* (Transformation|GetActorForwardVector) (* DeltaSeconds (Variables|Default|GetSpeed)))) false false))))

(fn ConstructionScript)