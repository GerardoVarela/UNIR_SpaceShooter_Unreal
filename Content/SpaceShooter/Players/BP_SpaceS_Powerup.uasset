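; BP_SpaceS_Powerup is a space shooter pickup that drifts in a straight line until the player collects it.
; It stores its forward vector at BeginPlay and moves along it every tick at Speed, without sweeping.
; Overlap with a "Player"-tagged BP_SpaceS_Character fires the OnPlayerPick dispatcher.
; The powerup's own bound event then destroys it after a short delay; no effect is applied here.
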(event Custom|PickEvent
  ;[0.15 0.15 0.15 0.5] Set Movement Direction
  (Utilities|FlowControl|Delay 0.1)
  (Actor|DestroyActor))

(event EventBeginPlay
  ;[0.15 0.15 0.15 0.5] Set Movement Direction
  (Variables|Default|SetMovementVector (Transformation|GetActorForwardVector))
  (EventDispatchers|BindEventtoOnPlayerPick (delegate Custom|PickEvent)))

(event Collision|EventActorBeginOverlap
  (params (OtherActor :type Actor%20Object%20Reference))
  ;[0.15 0.15 0.15 0.5] Overlap with Player
  (if (Actor|ActorHasTag OtherActor "Player")
    (Utilities|Casting|CastToBP_SpaceS_Character OtherActor)
    (Default|CallOnPlayerPick)))

(event EventTick
  (params (DeltaSeconds :type Float%20%28single-precision%29))
  ;[0.15 0.15 0.15 0.5] Move
  (CallFunction|Move DeltaSeconds))

(fn ConstructionScript)

(fn Move
  (params (DeltaTime :type Float%20%28double-precision%29))
  (Transformation|SetActorLocation (+ (Transformation|GetActorLocation) (* (* DeltaTime (Variables|Default|GetSpeed)) (Variables|Default|GetMovementVector))) false false))